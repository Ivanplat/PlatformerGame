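; Base world gate Blueprint that moves its root component through a timeline when PlayGateAnimation is called.
; The Open flag, only read here, selects Play or Reverse on GateAnimation and sets a sign multiplier.
; Each update adds the signed vector value as a cumulative, unswept local offset, rather than interpolating between fixed positions.
; A playing flag is raised at the start and cleared when the timeline finishes.
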(event `self.PlayGateAnimation`
  (set `self.AnimationgPlaying` true)
  (set `self.Multiplier` (select `bool` (`self.Open`) :`false` 1 :`true` -1))
  (if (not (`self.Open`))
    (bind (_direction _vectorvalue) (`Timeline|GateAnimation` :!label _label)
      (:`Update`
        (`SceneComponent.K2_AddLocalOffset` (`self.Root`) (* _vectorvalue (`self.Multiplier`)) false false))
      (:`Finished`
        (set `self.AnimationgPlaying` false)))
    (else
      (goto _label :!via `Reverse`))))

(fn `UserConstructionScript`)