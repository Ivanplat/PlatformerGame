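; Base Blueprint for an EBox world actor with an animated mesh that responds to an Enabled state.
; PlayEBoxAnimation plays or reverses a timeline based on Enabled, with a PlayingAnimation flag tracking the motion.
; Timeline updates add local pitch to StaticMesh incrementally, using a sign multiplier to set the direction.
; The Construction Script sets the light color and applies a dynamic M_BaseColor material instance to color the mesh.
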(event `self.PlayEBoxAnimation`
  (set `self.PlayingAnimation` true)
  (set `self.Multiply` (select `bool` (`self.Enabled`) :`false` 1 :`true` -1))
  (if (`self.Enabled`)
    (bind (_direction _rotation) (`Timeline|EBoxAnimation` :!label _label)
      (:`Update`
        (bind (_returnvalue_x _returnvalue_y) (`KismetMathLibrary.BreakVector` (* _rotation (`self.Multiply`))))
        (`SceneComponent.K2_AddLocalRotation` (`self.StaticMesh`) (`KismetMathLibrary.MakeRotator` 0.0 _returnvalue_y) false false))
      (:`Finished`
        (set `self.PlayingAnimation` false)))
    (else
      (goto _label :!via `Reverse`))))

(fn `UserConstructionScript`
  (locals (LDynamicMaterial :type "MaterialInstanceDynamic Object Reference"))
  (`self.SetLightColor`)
  (bind _returnvalue (`KismetMaterialLibrary.CreateDynamicMaterialInstance` "/Game/Assets/Materials/M_BaseColor.M_BaseColor" "123"))
  (set `local.LDynamicMaterial` _returnvalue)
  (`self.SetMeshMaterialColor` (`local.LDynamicMaterial`) (`self.Mesh`)))